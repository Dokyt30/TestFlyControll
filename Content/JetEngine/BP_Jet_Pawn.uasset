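; BP_Jet_Pawn is a player-controlled flying pawn with six-axis movement and two toggleable physics thrusters.
; Move inputs add linear velocity to the physics body mesh along the actor's forward, right and up vectors.
; Pitch, yaw and roll inputs apply local actor rotation directly, without torque or delta-time scaling.
; F toggles both thrusters; G doubles the stored thrust, initialized at BeginPlay, without limit and copies it to both.
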(event EventBeginPlay
  (Variables|Default|SetThrustStrength 1e+03))

(event Collision|EventActorBeginOverlap
  (params (OtherActor :type Actor%20Object%20Reference)))

(event EventTick
  (params (DeltaSeconds :type Float%20%28single-precision%29)))

(event Input|AxisEvents|InputAxisMoveForward
  (params (AxisValue :type Float%20%28single-precision%29))
  (Physics|SetPhysicsLinearVelocity (Variables|Default|GetBodyMesh) (* (Math|Vector|GetForwardVector (Transformation|GetActorRotation)) (* AxisValue 3.0)) true "None"))

(event Input|AxisEvents|InputAxisMoveRight
  (params (AxisValue :type Float%20%28single-precision%29))
  (Physics|SetPhysicsLinearVelocity (Variables|Default|GetBodyMesh) (* (Math|Vector|GetRightVector (Transformation|GetActorRotation)) (* AxisValue 3.0)) true "None"))

(event Input|AxisEvents|InputAxisMoveUp
  (params (AxisValue :type Float%20%28single-precision%29))
  (Physics|SetPhysicsLinearVelocity (Variables|Default|GetBodyMesh) (* (Math|Vector|GetUpVector (Transformation|GetActorRotation)) (* AxisValue 3.0)) true "None"))

(event Input|AxisEvents|InputAxisTurnPitch
  (params (AxisValue :type Float%20%28single-precision%29))
  (Transformation|AddActorLocalRotation (Math|Rotator|MakeRotator 0.0 AxisValue 0.0) false false))

(event Input|AxisEvents|InputAxisTurnYaw
  (params (AxisValue :type Float%20%28single-precision%29))
  (Transformation|AddActorLocalRotation (Math|Rotator|MakeRotator 0.0 0.0 AxisValue) false false))

(event Input|AxisEvents|InputAxisTurnRoll
  (params (AxisValue :type Float%20%28single-precision%29))
  (Transformation|AddActorLocalRotation (Math|Rotator|MakeRotator AxisValue 0.0 0.0) false false))

(event Input|KeyboardEvents|F
  (params (Key :type Key%20Structure))
  (:Pressed
    (Components|Activation|ToggleActive (Variables|Default|GetPhysicsThrusterR))
    (Components|Activation|ToggleActive (Variables|Default|GetPhysicsThrusterL))))

(event Input|KeyboardEvents|G
  (params (Key :type Key%20Structure))
  (:Pressed
    (Variables|Default|SetThrustStrength (* (Variables|Default|GetThrustStrength) 2.0))
    (Variables|/Script/Engine.PhysicsThrusterComponent|SetThrustStrength (Variables|Default|GetPhysicsThrusterR) (Variables|Default|GetThrustStrength))
    (Variables|/Script/Engine.PhysicsThrusterComponent|SetThrustStrength (Variables|Default|GetPhysicsThrusterL) (Variables|Default|GetThrustStrength))))

(fn ConstructionScript)